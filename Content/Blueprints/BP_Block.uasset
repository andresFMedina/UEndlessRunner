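; BP_Block is an endless-runner street segment with four obstacle lanes, coins and random buildings.
; On BeginPlay it randomises meshes, skips street lanes where a traced neighbouring block has a truck, and may put a coin in an empty lane.
; Street obstacles move every tick at frame-dependent speed; obstacle overlaps add hits, camera shake and immunity to non-immune players.
; Player overlap with OverlapBox makes the GameMode add a block, then this one self-destroys after a delay.
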(event OnComponentBeginOverlap(OverlapBox)
  (params (OverlappedComponent :type Primitive%20Component%20Object%20Reference) (OtherActor :type Actor%20Object%20Reference) (OtherComp :type Primitive%20Component%20Object%20Reference) (OtherBodyIndex :type Integer) (bFromSweep :type Boolean) (SweepResult :type Hit%20Result%20Structure%20%28by%20ref%29))
  (Utilities|Casting|CastToBP_ThirdPersonCharacter OtherActor)
  (bind _asbp_third_person_game_mode (Utilities|Casting|CastToBP_ThirdPersonGameMode (Game|GetGameMode)))
  (Default|AddBlock _asbp_third_person_game_mode true)
  (Utilities|FlowControl|Delay 5.0)
  (Actor|DestroyActor))

(event OnComponentBeginOverlap(Obstacle1)
  (params (OverlappedComponent :type Primitive%20Component%20Object%20Reference) (OtherActor :type Actor%20Object%20Reference) (OtherComp :type Primitive%20Component%20Object%20Reference) (OtherBodyIndex :type Integer) (bFromSweep :type Boolean) (SweepResult :type Hit%20Result%20Structure%20%28by%20ref%29))
  (bind _asbp_third_person_character (Utilities|Casting|CastToBP_ThirdPersonCharacter OtherActor))
  (CallFunction|HitPlayer _asbp_third_person_character))

(event OnComponentBeginOverlap(Obstacle2)
  (params (OverlappedComponent :type Primitive%20Component%20Object%20Reference) (OtherActor :type Actor%20Object%20Reference) (OtherComp :type Primitive%20Component%20Object%20Reference) (OtherBodyIndex :type Integer) (bFromSweep :type Boolean) (SweepResult :type Hit%20Result%20Structure%20%28by%20ref%29))
  (bind _asbp_third_person_character (Utilities|Casting|CastToBP_ThirdPersonCharacter OtherActor))
  (CallFunction|HitPlayer _asbp_third_person_character))

(event OnComponentBeginOverlap(Obstacle3)
  (params (OverlappedComponent :type Primitive%20Component%20Object%20Reference) (OtherActor :type Actor%20Object%20Reference) (OtherComp :type Primitive%20Component%20Object%20Reference) (OtherBodyIndex :type Integer) (bFromSweep :type Boolean) (SweepResult :type Hit%20Result%20Structure%20%28by%20ref%29))
  (bind _asbp_third_person_character (Utilities|Casting|CastToBP_ThirdPersonCharacter OtherActor))
  (CallFunction|HitPlayer _asbp_third_person_character))

(event OnComponentBeginOverlap(Obstacle4)
  (params (OverlappedComponent :type Primitive%20Component%20Object%20Reference) (OtherActor :type Actor%20Object%20Reference) (OtherComp :type Primitive%20Component%20Object%20Reference) (OtherBodyIndex :type Integer) (bFromSweep :type Boolean) (SweepResult :type Hit%20Result%20Structure%20%28by%20ref%29))
  (bind _asbp_third_person_character (Utilities|Casting|CastToBP_ThirdPersonCharacter OtherActor))
  (CallFunction|HitPlayer _asbp_third_person_character))

(event EventBeginPlay
  (bind _frontblock (CallFunction|CheckFrontBlock))
  (Utilities|IsValid _frontblock
    (:Is%20Valid
      (Variables|Default|SetSpawnLane2Car (!= (Variables|/Script/Engine.StaticMeshComponent|GetStaticMesh (Variables|BP_Block_C|GetObstacle2 _frontblock)) "/Game/AssetsvilleTown/Meshes/Vehicles/SM_veh_Truck_Merged_01.SM_veh_Truck_Merged_01"))
      (Variables|Default|SetSpawnLane3Car (!= (Variables|/Script/Engine.StaticMeshComponent|GetStaticMesh (Variables|BP_Block_C|GetObstacle3 _frontblock)) "/Game/AssetsvilleTown/Meshes/Vehicles/SM_veh_Truck_Merged_01.SM_veh_Truck_Merged_01")))
    (:Is%20Not%20Valid
      _))
  (CallFunction|SpawnObstacles)
  (CallFunction|SpawnCoins)
  (CallFunction|SpawnBuildings))

(event Collision|EventActorBeginOverlap
  (params (OtherActor :type Actor%20Object%20Reference)))

(event EventTick
  (params (DeltaSeconds :type Float%20%28single-precision%29))
  (CallFunction|MoveCars))

(fn ConstructionScript)

(fn SpawnObstacles
  (if (Variables|Default|GetisSpawningObstacles)
    (if (== (Math|Random|RandomIntegerinRange 0 1) 0)
      (Utilities|FlowControl|Sequence
        (:then_0
          (if (== (Math|Random|RandomIntegerinRange 0 1) 0)
            (Components|StaticMesh|SetStaticMesh (Variables|Default|GetObstacle1) (.OutItem (Utilities|Array|Random (Variables|Default|GetSidewalkMeshes))))))
        (:then_1
          (if (Variables|Default|GetSpawnLane2Car)
            (if (== (Math|Random|RandomIntegerinRange 0 1) 0)
              (Components|StaticMesh|SetStaticMesh (Variables|Default|GetObstacle2) (.OutItem (Utilities|Array|Random (Variables|Default|GetStreetMeshes)))))))
        (:then_2
          (if (Variables|Default|GetSpawnLane3Car)
            (if (== (Math|Random|RandomIntegerinRange 0 1) 0)
              (Components|StaticMesh|SetStaticMesh (Variables|Default|GetObstacle3) (.OutItem (Utilities|Array|Random (Variables|Default|GetStreetMeshes)))))))
        (:then_3
          (if (== (Math|Random|RandomIntegerinRange 0 1) 0)
            (Components|StaticMesh|SetStaticMesh (Variables|Default|GetObstacle4) (.OutItem (Utilities|Array|Random (Variables|Default|GetSidewalkMeshes))))))))))

(fn MoveCars
  (bind _obstacle2 (Variables|Default|GetObstacle2))
  (bind _obstacle3 (Variables|Default|GetObstacle3))
  (Transformation|SetWorldLocation _obstacle2 (+ (Transformation|GetWorldLocation _obstacle2) (* "0.000000,-1.000000,0.000000" 1e+01)) false false)
  (Transformation|SetWorldLocation _obstacle3 (+ (Transformation|GetWorldLocation _obstacle3) (* "0.000000,-1.000000,0.000000" 1e+01)) false false))

(fn CheckFrontBlock
  (bind _returnvalue (Transformation|GetActorLocation))
  (bind _outhit (Collision|LineTraceByChannel _returnvalue (+ _returnvalue (* (Transformation|GetActorRightVector) -4e+02)) "TraceTypeQuery1" false 0 "None"))
  (bind _asbp_block (Utilities|Casting|CastToBP_Block (.HitActor (Collision|BreakHitResult _outhit))))
  (return _asbp_block))

(fn SpawnCoins
  (Variables|Default|SetCoinLane (Math|Random|RandomIntegerinRange 0 3))
  (Utilities|IsValid (Variables|/Script/Engine.StaticMeshComponent|GetStaticMesh (Utilities|Select :Index (Variables|Default|GetCoinLane) :Option%200 (Variables|Default|GetObstacle1) :Option%201 (Variables|Default|GetObstacle2) :Option%202 (Variables|Default|GetObstacle3) :Option%203 (Variables|Default|GetObstacle4)))
    (:Is%20Not%20Valid
      (Game|SpawnActorfromClass "/Game/Blueprints/BP_Coin.BP_Coin_C" (Math|Transform|MakeTransform (Transformation|GetWorldLocation (Utilities|Select :Index (Variables|Default|GetCoinLane) :Option%200 (Variables|Default|GetObstacle1) :Option%201 (Variables|Default|GetObstacle2) :Option%202 (Variables|Default|GetObstacle3) :Option%203 (Variables|Default|GetObstacle4))) "0, 0, 0" "1.000000,1.000000,1.000000") "Undefined" 0 0))))

(fn HitPlayer
  (params (PlayerRef :type BP%20Third%20Person%20Character%20Object%20Reference))
  (if (not (Variables|/Game/ThirdPerson/Blueprints/BP_ThirdPersonCharacter.BP_ThirdPersonCharacter_C|GetImmune PlayerRef))
    (Math|Integer|IncrementInt (Variables|/Game/ThirdPerson/Blueprints/BP_ThirdPersonCharacter.BP_ThirdPersonCharacter_C|GetHits PlayerRef)
      (:%20%20
        (Variables|/Game/ThirdPerson/Blueprints/BP_ThirdPersonCharacter.BP_ThirdPersonCharacter_C|SetSpringArmInterSpeed PlayerRef 0.0)
        (Default|WaittoRemoveHit PlayerRef)
        (Game|Feedback|ClientStartCameraShake (Game|GetPlayerController 0) "/Game/Blueprints/CS_HitObject.CS_HitObject_C" 1.0 "CameraLocal" "0, 0, 0")
        (Default|Immunity PlayerRef)))))

(fn SpawnBuildings
  (Components|StaticMesh|SetStaticMesh (Variables|Default|GetBuilding1) (.OutItem (Utilities|Array|Random (Variables|Default|GetBuildMeshes))))
  (Components|StaticMesh|SetStaticMesh (Variables|Default|GetBuilding2) (.OutItem (Utilities|Array|Random (Variables|Default|GetBuildMeshes)))))